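; Flyable physics-driven ship that the first-person player boards through Interact and pilots with Enhanced Input.
; A thruster, aligned with the center of mass on BeginPlay, provides mass-scaled, tilt-compensated vertical thrust until forward thrust gets too high.
; Forward input eases a thrust value that drives engine audio RPM and, above a threshold, overrides linear velocity on Tick.
; Pitch, yaw and roll share a torque helper gated by that same threshold.
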(event Custom|OnShipUnoccupied
  (Variables|Default|SetOnShipOccupied false)
  (Variables|/Game/FirstPerson/Blueprints/BP_FirstPersonCharacter.BP_FirstPersonCharacter_C|SetCurrentShip (Variables|Default|GetPlayer) 0))

(event Input|EnhancedActionEvents|EnhancedInputActionIA_LeaveShip
  (params (ActionValue :type Boolean) (ElapsedSeconds :type Float%20%28double-precision%29) (TriggeredSeconds :type Float%20%28double-precision%29) (InputAction :type Input%20Action%20Object%20Reference :default "/Game/Input/Actions/IA_LeaveShip.IA_LeaveShip"))
  (:Started
    (Default|OnShipLeave (Variables|Default|GetPlayer))
    (Components|Activation|Deactivate (Variables|Default|GetPhysicsThruster))))

(event Input|EnhancedActionEvents|EnhancedInputActionIA_MoveShip
  (params (ActionValue :type Float%20%28double-precision%29) (ElapsedSeconds :type Float%20%28double-precision%29) (TriggeredSeconds :type Float%20%28double-precision%29) (InputAction :type Input%20Action%20Object%20Reference :default "/Game/Input/Actions/IA_MoveShip.IA_MoveShip"))
  (bind _physicsthruster (Variables|Default|GetPhysicsThruster))
  (:Triggered
    (if (<= (Variables|Default|GetForwardThrust) 3e+03)
      (Variables|/Script/Engine.PhysicsThrusterComponent|SetThrustStrength _physicsthruster (* (/ (* ActionValue (Variables|Default|GetUpDownThrustStrength)) (.z (Transformation|GetActorUpVector))) (Physics|GetMass (Variables|Default|GetSM_StarSparrow05))))))
  (:Completed
    (Variables|/Script/Engine.PhysicsThrusterComponent|SetThrustStrength _physicsthruster 0.0)))

(event Input|EnhancedActionEvents|EnhancedInputActionIA_Pitch
  (params (ActionValue :type Float%20%28double-precision%29) (ElapsedSeconds :type Float%20%28double-precision%29) (TriggeredSeconds :type Float%20%28double-precision%29) (InputAction :type Input%20Action%20Object%20Reference :default "/Game/Input/Actions/IA_Pitch.IA_Pitch"))
  ;[0.15 0.15 0.15 0.5] Pitch, Yaw, Roll
  (CallFunction|RotateShip (Math|Vector|GetRightVector (Variables|Default|GetSM_StarSparrow05)) (Variables|Default|GetUpDownTorqueStrength) ActionValue))

(event Input|EnhancedActionEvents|EnhancedInputActionIA_Yaw
  (params (ActionValue :type Float%20%28double-precision%29) (ElapsedSeconds :type Float%20%28double-precision%29) (TriggeredSeconds :type Float%20%28double-precision%29) (InputAction :type Input%20Action%20Object%20Reference :default "/Game/Input/Actions/IA_Yaw.IA_Yaw"))
  ;[0.15 0.15 0.15 0.5] Pitch, Yaw, Roll
  (CallFunction|RotateShip (Math|Vector|GetUpVector (Variables|Default|GetSM_StarSparrow05)) (Variables|Default|GetYawTorqueStrength) ActionValue))

(event Input|EnhancedActionEvents|EnhancedInputActionIA_Roll
  (params (ActionValue :type Float%20%28double-precision%29) (ElapsedSeconds :type Float%20%28double-precision%29) (TriggeredSeconds :type Float%20%28double-precision%29) (InputAction :type Input%20Action%20Object%20Reference :default "/Game/Input/Actions/IA_Roll.IA_Roll"))
  ;[0.15 0.15 0.15 0.5] Pitch, Yaw, Roll
  (CallFunction|RotateShip (Math|Vector|GetForwardVector (Variables|Default|GetSM_StarSparrow05)) (Variables|Default|GetRollTorqueStrength) ActionValue))

(event Input|EnhancedActionEvents|EnhancedInputActionIA_ForwardBackward
  (params (ActionValue :type Float%20%28double-precision%29) (ElapsedSeconds :type Float%20%28double-precision%29) (TriggeredSeconds :type Float%20%28double-precision%29) (InputAction :type Input%20Action%20Object%20Reference :default "/Game/Input/Actions/IA_ForwardBackward.IA_ForwardBackward"))
  ;[0.15 0.15 0.15 0.5] Forward
  (Utilities|FlowControl|Sequence
    (:then_0
      (if (>= ActionValue 0.0)
        (Variables|Default|SetTargetLerpAlpha 1.0)
        (else
          (Variables|Default|SetTargetLerpAlpha 0.0)))
      (bind _output_get (Variables|Default|SetForwardThrust (Math|Interpolation|FInterpTo (Variables|Default|GetForwardThrust) (Math|Float|Lerp 0.0 (Variables|Default|GetMaxForwardThrust) (Variables|Default|GetTargetLerpAlpha)) (Utilities|Time|GetWorldDeltaSeconds) 1.0)))
      (Audio|Parameter|SetFloatParameter (Variables|Default|GetAudioCurveSource) "RPM" (Math|Float|MapRangeClamped (Math|Float|Absolute(Float) _output_get) 0.0 5e+03 0.0 1.0) :!class /Script/Engine.AudioComponent))
    (:then_1
      (Variables|Default|SetForwardMoveVector (* (Math|Vector|GetForwardVector (Variables|Default|GetSM_StarSparrow05)) (Variables|Default|GetForwardThrust))))))

(event EventBeginPlay
  (bind _sm_starsparrow05 (Variables|Default|GetSM_StarSparrow05))
  (bind _physicsthruster (Variables|Default|GetPhysicsThruster))
  (bind _sm_starsparrow05_2 (Variables|Default|GetSM_StarSparrow05))
  (bind _returnvalue (Transformation|GetWorldLocation _physicsthruster))
  (bind _returnvalue_2 (Physics|GetCenterOfMass _sm_starsparrow05_2 "None"))
  (bind _returnvalue_3 (Transformation|GetWorldRotation _sm_starsparrow05_2))
  (bind _returnvalue_4 (Class|KismetMathLibrary|NegateRotator _returnvalue_3))
  (bind _returnvalue_5 (- _returnvalue _returnvalue_2))
  (bind _returnvalue_6 (Math|Vector|RotateVector _returnvalue_5 _returnvalue_4))
  (bind _asbp_first_person_character (Utilities|Casting|CastToBP_FirstPersonCharacter (Game|GetPlayerCharacter 0)))
  (Variables|Default|SetPlayer _asbp_first_person_character)
  (Variables|Default|SetShipStaticMesh _sm_starsparrow05)
  (Class|PrimitiveComponent|SetCenterOfMass _sm_starsparrow05 (Math|Vector|MakeVector (.x _returnvalue_6) (.y _returnvalue_6) 0.0) "None"))

(event Collision|EventActorBeginOverlap
  (params (OtherActor :type Actor%20Object%20Reference)))

(event EventInteract
  (bind _player (Variables|Default|GetPlayer))
  (if (not (Variables|Default|GetOnShipOccupied))
    (Variables|Default|SetOnShipOccupied true)
    (Variables|/Game/FirstPerson/Blueprints/BP_FirstPersonCharacter.BP_FirstPersonCharacter_C|SetCurrentShip _player self)
    (Default|OnShipOccupied _player)
    (Components|Activation|Activate (Variables|Default|GetPhysicsThruster) false)
    (Components|Activation|Activate (Variables|Default|GetAudioCurveSource) false)))

(event EventTick
  (params (DeltaSeconds :type Float%20%28single-precision%29))
  ;[0.15 0.15 0.15 0.5] Move Forward
  (if (>= (Variables|Default|GetForwardThrust) 2e+02)
    (Physics|SetPhysicsLinearVelocity (Variables|Default|GetSM_StarSparrow05) (Variables|Default|GetForwardMoveVector) false "None")))

(fn ConstructionScript)

(fn RotateShip
  (params (Origin :type Vector) (Torque%20value :type Float%20%28double-precision%29) (Input%20value :type Float%20%28double-precision%29))
  (if (>= (Variables|Default|GetForwardThrust) 2e+02)
    (Class|PrimitiveComponent|AddTorqueinDegrees (Variables|Default|GetSM_StarSparrow05) (* Origin (* Torque%20value Input%20value)) "None" true)))