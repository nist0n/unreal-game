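; BP_QuestGiver is a quest pickup actor that grants its Quest class on overlap with its sphere.
; On any overlap it gets the first player controller's quest component through a message call, adds the quest, then destroys itself.
; Its widget shows the icon and name from the quest's class defaults.
; RotateTowardPlayer can turn the widget toward the player's head, and a looping timer is marked as cosmetic only.
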(event OnComponentBeginOverlap(Sphere)
  (params (OverlappedComponent :type Primitive%20Component%20Object%20Reference) (OtherActor :type Actor%20Object%20Reference) (OtherComp :type Primitive%20Component%20Object%20Reference) (OtherBodyIndex :type Integer) (bFromSweep :type Boolean) (SweepResult :type Hit%20Result%20Structure%20%28by%20ref%29))
  ;[0.005208 0.005208 0.005208 0.5] Handling Overlap Event
  (Utilities|FlowControl|Sequence
    (:then_0
      (bind _returnvalue (Class|QuestInterface|GetQuestComponent(Message) (Game|GetPlayerController 0)))
      (bind _output_get (Variables|Default|SetQuestComponent _returnvalue))
      (Utilities|IsValid _output_get
        (:Is%20Valid
          (Class|QuestComponent|AddQuest _output_get (Variables|Default|GetQuest)))))
    (:then_1
      (Actor|DestroyActor))))

(event EventBeginPlay
  (CallFunction|SetWidgetIcon)
  ;[0 0.5439 1] Cosmetics Only - Can be safely Removed!
  (Utilities|Time|SetTimerbyEvent (EventDispatchers|CreateEvent :!event RotateTowardPlayer) 0.5 true))

(fn ConstructionScript)

(fn SetWidgetIcon
  (bind _quest (Variables|Default|GetQuest))
  (bind (_name _icon) (Utilities|GetClassDefaults _quest))
  (bind _aswi_quest_item (Utilities|Casting|CastToWI_QuestItem (UserInterface|GetWidget (Variables|Default|GetWidget))))
  (Default|SetProperties _aswi_quest_item _icon _name))

(fn RotateTowardPlayer
  (bind _widget (Variables|Default|GetWidget))
  (Transformation|SetWorldRotation _widget (Math|Rotator|FindLookatRotation (Transformation|GetWorldLocation _widget) (Transformation|GetSocketLocation (Variables|/Script/Engine.Character|GetMesh (Game|GetPlayerCharacter 0)) "head")) false false))