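; Quest-giver NPC that hands the player a crystal fetch quest and completes it when the player returns with the item.
; On first Interact it adds its QuestClass to the first-person character's quest component and sets QuestGiven.
; Later interactions, while that quest is Active, check the inventory for the hardcoded DA_QuestCrystal, then either mark it Completed or show a reminder.
; Feedback uses Russian on-screen text, plus a sound on give and completion.
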(event EventBeginPlay)

(event Collision|EventActorBeginOverlap
  (params (OtherActor :type Actor%20Object%20Reference)))

(event EventTick
  (params (DeltaSeconds :type Float%20%28single-precision%29)))

(event EventInteract
  (bind _asbp_first_person_character (Utilities|Casting|CastToBP_FirstPersonCharacter (Game|Player|GetPlayerPawn 0)))
  (bind _returnvalue (Class|QuestInterface|GetQuestComponent _asbp_first_person_character))
  (if (Variables|Default|GetbQuestGiven)
    (if (Utilities|Enum|Equal(Enum) (Class|QuestComponent|GetQuestStatus _returnvalue (.Id (Utilities|GetClassDefaults (Variables|Default|GetQuestClass)))) "Active")
      (bind _returnvalue_2 (Class|QuestInterface|GetInventoryComponent(Message) _asbp_first_person_character))
      (if (Class|InventoryComponent|HasItem _returnvalue_2 "/Game/Blueprints/Quests/Items/DA_QuestCrystal.DA_QuestCrystal")
        (Class|QuestComponent|UpdateQuestStatus (Variables|/Game/Blueprints/BP_FirstPersonCharacter.BP_FirstPersonCharacter_C|GetQuest _asbp_first_person_character) (Variables|Default|GetQuestClass) "Completed")
        (Development|PrintText "Квест выполнен")
        (Audio|PlaySound2D "/Game/Audio/Pickup_Gold_00_Cue.Pickup_Gold_00_Cue" 1.0 1.0 0.0 0 0)
        (else
          (Development|PrintText "Сначала найди кристалл"))))
    (else
      (Class|QuestComponent|AddQuest _returnvalue (Variables|Default|GetQuestClass))
      (Variables|Default|SetbQuestGiven true)
      (Development|PrintText "Принеси кристалл")
      (Audio|PlaySound2D "/Game/Audio/Pickup_Gold_00_Cue.Pickup_Gold_00_Cue" 1.0 1.0 0.0 0 0))))

(fn ConstructionScript)