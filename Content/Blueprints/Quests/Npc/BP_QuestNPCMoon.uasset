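; Quest-giver NPC that hands the player a quest to visit the Moon.
; On first Interact it adds QuestClass to the quest component of the player's BP_FirstPersonCharacter, sets QuestGiven, prints the task in Russian and plays a pickup sound.
; Later interactions look up the quest status by the class-default Id and print a reminder while Active, otherwise a completion message.
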(event EventBeginPlay)

(event Collision|EventActorBeginOverlap
  (params (OtherActor :type Actor%20Object%20Reference)))

(event EventTick
  (params (DeltaSeconds :type Float%20%28single-precision%29)))

(event EventInteract
  (bind _asbp_first_person_character (Utilities|Casting|CastToBP_FirstPersonCharacter (Game|Player|GetPlayerPawn 0)))
  (bind _returnvalue (Class|QuestInterface|GetQuestComponent _asbp_first_person_character))
  (if (Variables|Default|GetbQuestGiven)
    (if (Utilities|Enum|Equal(Enum) (Class|QuestComponent|GetQuestStatus _returnvalue (.Id (Utilities|GetClassDefaults (Variables|Default|GetQuestClass)))) "Active")
      (Development|PrintText "Ты ещё не был на луне")
      (else
        (Development|PrintText "Квест завершён")))
    (else
      (Class|QuestComponent|AddQuest _returnvalue (Variables|Default|GetQuestClass))
      (Variables|Default|SetbQuestGiven true)
      (Development|PrintText "Побывай на луне")
      (Audio|PlaySound2D "/Game/Audio/Pickup_Gold_00_Cue.Pickup_Gold_00_Cue" 1.0 1.0 0.0 0 0))))

(fn ConstructionScript)