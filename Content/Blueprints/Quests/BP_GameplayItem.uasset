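; BP_GameplayItem is a pickup actor that adds its item to the player's inventory on overlap.
; On BeginPlay it fills its quest item widget with the item's icon and name, then starts a cosmetic looping timer.
; On sphere overlap it gets player 0's inventory component through a message call, adds one item and destroys itself.
; A RotateTowardPlayer function turns the widget toward the player's head socket.
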(event OnComponentBeginOverlap(Sphere)
  (params (OverlappedComponent :type Primitive%20Component%20Object%20Reference) (OtherActor :type Actor%20Object%20Reference) (OtherComp :type Primitive%20Component%20Object%20Reference) (OtherBodyIndex :type Integer) (bFromSweep :type Boolean) (SweepResult :type Hit%20Result%20Structure%20%28by%20ref%29))
  ;[0.005208 0.005208 0.005208 0.5] Handling Overlap Event
  (Utilities|FlowControl|Sequence
    (:then_0
      ;;[0.005208 0.005208 0.005208 0.5] Currently The Item would be automatically added to inventory when you collide with the actor
      (bind _returnvalue (Class|QuestInterface|GetInventoryComponent(Message) (Game|GetPlayerController 0)))
      (bind _output_get (Variables|Default|SetInventory _returnvalue))
      (Utilities|IsValid _output_get
        (:Is%20Valid
          (Class|InventoryComponent|AddtoInventory _output_get (Variables|Default|GetItem) 1))))
    (:then_1
      (Utilities|FlowControl|Delay 0.0)
      (Actor|DestroyActor))))

(event EventBeginPlay
  (bind _item (Variables|Default|GetItem))
  (bind _aswi_quest_item (Utilities|Casting|CastToWI_QuestItem (UserInterface|GetWidget (Variables|Default|GetWidget))))
  (Default|SetProperties _aswi_quest_item (Variables|/Script/QuestSystem.GameplayItemData|GetIcon _item) (Variables|/Script/QuestSystem.GameplayItemData|GetName _item))
  ;[0 0.5439 1] Cosmetics Only - Can be safely Removed!
  (Utilities|Time|SetTimerbyEvent (EventDispatchers|CreateEvent :!event RotateTowardPlayer) 0.5 true))

(fn ConstructionScript)

(fn RotateTowardPlayer
  (bind _widget (Variables|Default|GetWidget))
  (Transformation|SetWorldRotation _widget (Math|Rotator|FindLookatRotation (Transformation|GetWorldLocation _widget) (Transformation|GetSocketLocation (Variables|/Script/Engine.Character|GetMesh (Game|GetPlayerCharacter 0)) "head")) false false))