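; Game instance for the minimalistic menu that saves and loads general, graphics and audio settings through a save game object.
; LoadGame caches the slot's existing save as SGMinimalisticMenu, or creates a new BP_MinimalisticMenuSaveGame when none exists.
; SaveGame copies the three settings structs into that cached object and writes it to the named slot, doing nothing if the object is invalid.
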(fn SaveGame
  (params (SlotName :type String) (Struc_General :type Struc%20General%20Structure) (Struc_Graphics :type Struc%20Graphics%20Structure) (Struc_Audio :type Struc%20Audio%20Structure))
  (bind _sg_minimalisticmenu (Variables|Default|GetSG_MinimalisticMenu)
    (:then
      (Variables|/Game/MinimalisticMenu/Blueprints/SaveGame/BP_MinimalisticMenuSaveGame.BP_MinimalisticMenuSaveGame_C|SetStruc_General _sg_minimalisticmenu Struc_General)
      (Variables|/Game/MinimalisticMenu/Blueprints/SaveGame/BP_MinimalisticMenuSaveGame.BP_MinimalisticMenuSaveGame_C|SetStruc_Graphics _sg_minimalisticmenu Struc_Graphics)
      (Variables|/Game/MinimalisticMenu/Blueprints/SaveGame/BP_MinimalisticMenuSaveGame.BP_MinimalisticMenuSaveGame_C|SetStruc_Audio _sg_minimalisticmenu Struc_Audio)
      (SaveGame|SaveGametoSlot (Variables|Default|GetSG_MinimalisticMenu) SlotName))
    (:else)))

(fn LoadGame
  (params (SlotName :type String))
  (bind _returnvalue (SaveGame|DoesSaveGameExist SlotName))
  (if _returnvalue
    (bind _returnvalue_2 (SaveGame|LoadGamefromSlot SlotName))
    (bind _asbp_minimalistic_menu_save_game (Utilities|Casting|CastToBP_MinimalisticMenuSaveGame _returnvalue_2))
    (Variables|Default|SetSG_MinimalisticMenu _asbp_minimalistic_menu_save_game)
    (else
      (bind _returnvalue_3 (SaveGame|CreateSaveGameObject "/Game/MinimalisticMenu/Blueprints/SaveGame/BP_MinimalisticMenuSaveGame.BP_MinimalisticMenuSaveGame_C"))
      (Variables|Default|SetSG_MinimalisticMenu _returnvalue_3))))