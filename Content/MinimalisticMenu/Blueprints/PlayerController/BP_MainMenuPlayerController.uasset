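; Main menu player controller that loads saved settings through the Minimalistic Menu game instance on BeginPlay and applies them.
; Graphics quality values become scalability console commands through the ExecuteCC helper.
; Audio sets SCM_Master as base mix and overrides Ambient and SoundFX class volumes, each multiplied by the saved Voice value.
; General settings only copy the saved difficulty into a variable, after validity checks.
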(event EventBeginPlay
  (bind _asgi_minimalistic_menu (Utilities|Casting|CastToBP_MinimalisticMenuGameInstance (Game|GetGameInstance)))
  (bind _output_get (Variables|Default|SetAs%20GI%20Minimalistic%20Menu _asgi_minimalistic_menu))
  (Default|LoadGame _output_get "MM_SG1")
  (CallFunction|LoadGeneralSet)
  (CallFunction|LoadGraphicsSet)
  (CallFunction|LoadAudioSet))

(fn ConstructionScript)

(fn LoadGraphicsSet
  (bind _as_gi_minimalistic_menu (Variables|Default|GetAs%20GI%20Minimalistic%20Menu))
  (bind _sg_minimalisticmenu (Variables|/Game/MinimalisticMenu/Blueprints/GameInstance/BP_MinimalisticMenuGameInstance.BP_MinimalisticMenuGameInstance_C|GetSG_MinimalisticMenu _as_gi_minimalistic_menu))
  (bind _struc_graphics (Variables|/Game/MinimalisticMenu/Blueprints/SaveGame/BP_MinimalisticMenuSaveGame.BP_MinimalisticMenuSaveGame_C|GetStruc_Graphics _sg_minimalisticmenu))
  (bind (_viewdistance _anti_aliasing _postprocessing _shadow _globalillumination _reflection _textures _effects _foliage _shading _lansdscape) (Utilities|Struct|BreakStruc_Graphics _struc_graphics))
  (CallFunction|ExecuteCC "sg.ViewDistanceQuality" _viewdistance)
  (CallFunction|ExecuteCC "sg.AntiAliasingQuality" _anti_aliasing)
  (CallFunction|ExecuteCC "sg.PostProcessQuality" _postprocessing)
  (CallFunction|ExecuteCC "sg.ShadowQuality" _shadow)
  (CallFunction|ExecuteCC "sg.GlobalIlluminationQuality" _globalillumination)
  (CallFunction|ExecuteCC "sg.ReflectionQuality" _reflection)
  (CallFunction|ExecuteCC "sg.TextureQuality" _textures)
  (CallFunction|ExecuteCC "sg.EffectsQuality" _effects)
  (CallFunction|ExecuteCC "sg.FoliageQuality" _foliage)
  (CallFunction|ExecuteCC "sg.ShadingQuality" _shading)
  (CallFunction|ExecuteCC "sg.LandscapeQuality" _lansdscape))

(fn LoadAudioSet
  (bind _as_gi_minimalistic_menu (Variables|Default|GetAs%20GI%20Minimalistic%20Menu))
  (bind _sg_minimalisticmenu (Variables|/Game/MinimalisticMenu/Blueprints/GameInstance/BP_MinimalisticMenuGameInstance.BP_MinimalisticMenuGameInstance_C|GetSG_MinimalisticMenu _as_gi_minimalistic_menu))
  (bind _struc_audio (Variables|/Game/MinimalisticMenu/Blueprints/SaveGame/BP_MinimalisticMenuSaveGame.BP_MinimalisticMenuSaveGame_C|GetStruc_Audio _sg_minimalisticmenu))
  (bind (_ambient _soundfx _voice) (Utilities|Struct|BreakStruc_Audio _struc_audio))
  (Class|GameplayStatics|SetBaseSoundMix "/Game/MinimalisticMenu/Audio/SoundClass/SCM_Master.SCM_Master")
  (Audio|SetSoundMixClassOverride "/Game/MinimalisticMenu/Audio/SoundClass/SCM_Master.SCM_Master" "/Game/MinimalisticMenu/Audio/SoundClass/SC_Ambient.SC_Ambient" (* _voice _ambient) 1.0 0.0 true)
  (Audio|SetSoundMixClassOverride "/Game/MinimalisticMenu/Audio/SoundClass/SCM_Master.SCM_Master" "/Game/MinimalisticMenu/Audio/SoundClass/SC_SoundFX.SC_SoundFX" (* _voice _soundfx) 1.0 0.0 true))

(fn ExecuteCC
  (params (Command :type String) (Value :type Integer))
  (Development|ExecuteConsoleCommand (Utilities|String|Append Command " " (Utilities|String|ToString(Integer) Value)) 0))

(fn LoadGeneralSet
  (bind _as_gi_minimalistic_menu (Variables|Default|GetAs%20GI%20Minimalistic%20Menu)
    (:then
      (bind _sg_minimalisticmenu (Variables|/Game/MinimalisticMenu/Blueprints/GameInstance/BP_MinimalisticMenuGameInstance.BP_MinimalisticMenuGameInstance_C|GetSG_MinimalisticMenu _as_gi_minimalistic_menu)
        (:then
          (Variables|Default|SetDifficulty (.difficulty (Variables|/Game/MinimalisticMenu/Blueprints/SaveGame/BP_MinimalisticMenuSaveGame.BP_MinimalisticMenuSaveGame_C|GetStruc_General _sg_minimalisticmenu))))
        (:else)))
    (:else)))